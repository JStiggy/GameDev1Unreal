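; Javelin projectile actor that damages enemy ostriches and expires on a lifespan timer if it strikes none.
; A Box overlap with an EnemyOstrich calls OstrichHit, which applies damage, sets a fleeing ostrich's PlayerPosition to the javelin's location, and destroys the javelin.
; A blocking hit on the Box shortens the remaining lifespan, and both impact paths play the spear hit sound at the javelin's location.
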(event OnComponentBeginOverlap(Box)
  (params (OverlappedComponent :type Primitive%20Component%20Object%20Reference) (OtherActor :type Actor%20Object%20Reference) (OtherComp :type Primitive%20Component%20Object%20Reference) (OtherBodyIndex :type Integer) (bFromSweep :type Boolean) (SweepResult :type Hit%20Result%20Structure%20%28by%20ref%29))
  (bind _asenemy_ostrich (Utilities|Casting|CastToEnemyOstrich OtherActor))
  (CallFunction|OstrichHit _asenemy_ostrich)
  (Audio|PlaySoundatLocation "/Game/Audio/SFX/SpearHit_Cue.SpearHit_Cue" (Transformation|GetActorLocation)))

(event OnComponentHit(Box)
  (params (HitComponent :type Primitive%20Component%20Object%20Reference) (OtherActor :type Actor%20Object%20Reference) (OtherComp :type Primitive%20Component%20Object%20Reference) (NormalImpulse :type Vector :default "0, 0, 0") (Hit :type Hit%20Result%20Structure%20%28by%20ref%29))
  (Actor|SetLifeSpan 2.0)
  (Audio|PlaySoundatLocation "/Game/Audio/SFX/SpearHit_Cue.SpearHit_Cue" (Transformation|GetActorLocation)))

(event EventBeginPlay
  (Actor|SetLifeSpan 1e+01))

(fn ConstructionScript)

(fn OstrichHit
  (params (NewParam :type Enemy%20Ostrich%20Object%20Reference))
  (Default|Damage NewParam 2)
  (if (Variables|/Game/Blueprints/EnemyOstrich.EnemyOstrich_C|GetFleeing NewParam)
    (Variables|/Game/Blueprints/EnemyOstrich.EnemyOstrich_C|SetPlayerPosition NewParam (Transformation|GetActorLocation)))
  (Actor|DestroyActor))