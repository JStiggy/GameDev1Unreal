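; Lever is a one-shot interactable that acts as a respawn checkpoint for the first-person player.
; On its first Interact it saves the player's current transform as the character's RespawnLocation and plays a breaker switch sound.
; It also toggles the visibility of its Light and sets Activated so later interactions do nothing.
; The lever animation is still a debug print placeholder.
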(event EventBeginPlay)

(event Collision|EventActorBeginOverlap
  (params (OtherActor :type Actor%20Object%20Reference)))

(event EventTick
  (params (DeltaSeconds :type Float%20%28single-precision%29)))

(event EventInteract
  (bind _returnvalue (Game|GetPlayerCharacter 0))
  (if (not (Variables|Default|GetActivated))
    (bind _asfirst_person_character (Utilities|Casting|CastToFirstPersonCharacter _returnvalue))
    (Variables|/Game/FirstPersonBP/Blueprints/FirstPersonCharacter.FirstPersonCharacter_C|SetRespawnLocation _asfirst_person_character (Transformation|GetActorTransform _returnvalue))
    (Audio|PlaySound2D "/Game/Audio/SFX/BreakerSwitch.BreakerSwitch")
    (Development|PrintString "Play Lever Anim Here")
    (Rendering|ToggleVisibility (Variables|/Script/Engine.Light|GetLightComponent (Variables|Default|GetLight)) false)
    (Variables|Default|SetActivated true)))

(fn ConstructionScript
  (|CallParentFunction))