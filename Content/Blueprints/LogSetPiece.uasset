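; LogSetPiece is an interactable spot where the player places a carried log.
; It starts with ChoppedLog hidden, and Interact checks either hand of the FirstPersonCharacter for a Log_Item.
; A one-time placement reveals the log, sets LogPlaced and disables PreLogCollision.
; It then empties both hands, whichever held the log, clearing their items and meshes and refreshing hand animations.
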(event EventBeginPlay
  (bind _choppedlog (Variables|Default|GetChoppedLog))
  (Rendering|SetVisibility _choppedlog false false)
  (Development|SetHiddeninGame _choppedlog true false))

(event EventInteract
  (bind _choppedlog (Variables|Default|GetChoppedLog))
  (bind _asfirst_person_character (Utilities|Casting|CastToFirstPersonCharacter (Game|GetPlayerCharacter 0)))
  (if (and (or (Utilities|ClassIsChildOf (Utilities|GetClass (Variables|/Game/FirstPersonBP/Blueprints/FirstPersonCharacter.FirstPersonCharacter_C|GetL_Item _asfirst_person_character)) "/Game/Blueprints/Pickup_Items/Log_Item.Log_Item_C") (Utilities|ClassIsChildOf (Utilities|GetClass (Variables|/Game/FirstPersonBP/Blueprints/FirstPersonCharacter.FirstPersonCharacter_C|GetR_Item _asfirst_person_character)) "/Game/Blueprints/Pickup_Items/Log_Item.Log_Item_C")) (not (Variables|Default|GetLogPlaced)))
    (Rendering|SetVisibility _choppedlog true false)
    (Development|SetHiddeninGame _choppedlog false false)
    (Variables|Default|SetLogPlaced true)
    (Collision|SetCollisionEnabled (Variables|Default|GetPreLogCollision) "NoCollision")
    (bind _asfirst_person_character_2 (Utilities|Casting|CastToFirstPersonCharacter (Game|GetPlayerCharacter 0)))
    (Class|SkinnedMeshComponent|SetSkeletalMesh (Variables|/Game/FirstPersonBP/Blueprints/FirstPersonCharacter.FirstPersonCharacter_C|GetL_Item_Skeletal _asfirst_person_character_2) 0 true)
    (Class|SkinnedMeshComponent|SetSkeletalMesh (Variables|/Game/FirstPersonBP/Blueprints/FirstPersonCharacter.FirstPersonCharacter_C|GetR_Item_Skeletal _asfirst_person_character_2) 0 true)
    (Variables|/Game/FirstPersonBP/Blueprints/FirstPersonCharacter.FirstPersonCharacter_C|SetL_Item _asfirst_person_character_2 0)
    (Variables|/Game/FirstPersonBP/Blueprints/FirstPersonCharacter.FirstPersonCharacter_C|SetR_Item _asfirst_person_character_2 0)
    (Default|HandAnim _asfirst_person_character_2 (Variables|/Game/FirstPersonBP/Blueprints/FirstPersonCharacter.FirstPersonCharacter_C|GetMesh_L _asfirst_person_character_2))
    (Default|HandAnim _asfirst_person_character_2 (Variables|/Game/FirstPersonBP/Blueprints/FirstPersonCharacter.FirstPersonCharacter_C|GetMesh_R _asfirst_person_character_2))))

(fn ConstructionScript
  (|CallParentFunction))