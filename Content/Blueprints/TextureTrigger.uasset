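; A trigger actor that shows its texture on the first-person HUD when the player character walks into its box.
; The overlap swaps the HUD's DisplayTexture and enables input on the actor, so releasing the left mouse button then destroys it.
; On destruction it restores the crosshair texture, but only if the HUD still displays this trigger's texture.
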(event OnComponentBeginOverlap(Box)
  (params (OverlappedComponent :type Primitive%20Component%20Object%20Reference) (OtherActor :type Actor%20Object%20Reference) (OtherComp :type Primitive%20Component%20Object%20Reference) (OtherBodyIndex :type Integer) (bFromSweep :type Boolean) (SweepResult :type Hit%20Result%20Structure%20%28by%20ref%29))
  (if (== OtherActor (Game|GetPlayerCharacter 0))
    (bind _asfirst_person_hud (Utilities|Casting|CastToFirstPersonHUD (HUD|GetHUD (Game|GetPlayerController 0))))
    (Variables|/Game/FirstPersonBP/Blueprints/FirstPersonHUD.FirstPersonHUD_C|SetDisplayTexture _asfirst_person_hud (Variables|Default|GetDisplayTexture))
    (Input|EnableInput (Game|GetPlayerController 0))))

(event EventDestroyed
  ;[1 1 1] Put the original texture back
  (if (== (Variables|Default|GetDisplayTexture) (Variables|/Game/FirstPersonBP/Blueprints/FirstPersonHUD.FirstPersonHUD_C|GetDisplayTexture (stale OnComponentBeginOverlap(Box) _asfirst_person_hud)))
    (Variables|/Game/FirstPersonBP/Blueprints/FirstPersonHUD.FirstPersonHUD_C|SetDisplayTexture (stale OnComponentBeginOverlap(Box) _asfirst_person_hud) "/Game/FirstPerson/Textures/FirstPersonCrosshair.FirstPersonCrosshair")))

(event Input|MouseEvents|LeftMouseButton
  (params (Key :type Key%20Structure :default "AnyKey"))
  (:Released
    (Actor|DestroyActor)))

(fn ConstructionScript)