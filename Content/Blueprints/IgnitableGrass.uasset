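; IgnitableGrass is a grass actor that catches fire, spreads it to nearby grass and makes enemy ostriches flee.
; Ignite shows the fire mesh, plays looked-up fire audio and limits the actor's lifespan.
; It then sets delayed Ignite timers on unlit grass within SpreadDistance, chaining the spread.
; While burning, Tick refreshes the flee state and timer on every EnemyOstrich in the level, regardless of distance.
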(event EventTick
  (params (DeltaSeconds :type Float%20%28single-precision%29))
  (if (Variables|Default|GetOnFire)
    (bind _outactors (Actor|GetAllActorsOfClass "/Game/Blueprints/EnemyOstrich.EnemyOstrich_C"))
    (for _array_element _outactors
      (Variables|/Game/Blueprints/EnemyOstrich.EnemyOstrich_C|SetFleeing _array_element true)
      (Variables|/Game/Blueprints/EnemyOstrich.EnemyOstrich_C|SetFleeTimer _array_element 2e+01))))

(fn ConstructionScript)

(fn Ignite
  (bind _firelowpoly (Variables|Default|GetFireLowPoly))
  (if (not (Variables|Default|GetOnFire))
    (Actor|SetLifeSpan 15.0)
    (Rendering|SetVisibility _firelowpoly true false)
    (Development|SetHiddeninGame _firelowpoly false false)
    (Variables|Default|SetOnFire true)
    (bind _returnvalue (AddComponent|AddAudioComponent false))
    (bind _output_get (Variables|Default|SetFire _returnvalue))
    (Audio|Components|Audio|SetSound _output_get "/Game/Audio/SFX/BigFire_Cue.BigFire_Cue")
    (Audio|Components|Audio|Play _output_get 0.0)
    (bind _outactors (Actor|GetAllActorsOfClass "IgnitableGrass_C"))
    (for _array_element _outactors
      (if (and (<= (Transformation|GetDistanceTo _array_element) (Variables|Default|GetSpreadDistance)) (not (Variables|IgnitableGrass_C|GetOnFire _array_element)))
        (Utilities|Time|SetTimerbyFunctionName _array_element "Ignite" (Variables|Default|GetFire%20Delay))))))