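; Ostrich enemy whose AI runs on Tick with state flags and navmesh moves, roaring on detection and death.
; It wanders until the player enters its view cone, then chases using line traces, falls back to the last known position, and launches the player up close (damage is a placeholder).
; Nearby ostriches share alerts and pool health into morale; low morale triggers fleeing, with health restored after a timer.
; Taking damage knocks it back and triggers pursuit.
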(event EventTick
  (params (DeltaSeconds :type Float%20%28single-precision%29))
  (if (> (Variables|Default|GetHealth) 0)
    (if (not (Variables|Default|GetFleeing))
      (Utilities|FlowControl|Sequence
        (:then_0
          (CallFunction|Wander DeltaSeconds))
        (:then_1
          (CallFunction|EnemyDetection))
        (:then_2
          (CallFunction|PursueVisibleEnemy DeltaSeconds))
        (:then_3
          (CallFunction|PursueLastKnownLocation DeltaSeconds))
        (:then_4
          (CallFunction|CalculateMorale)))
      (else
        (Utilities|FlowControl|Sequence
          (:then_0
            (CallFunction|EnemyDetection))
          (:then_1
            (CallFunction|Wander DeltaSeconds))
          (:then_2
            (CallFunction|CalculateFleeTime DeltaSeconds))
          (:then_3
            (CallFunction|Flee)))))
    (else
      (Audio|Components|Audio|Play (Variables|Default|GetOstricheNoise) 0.0)
      (Actor|DestroyActor))))

(event EventBeginPlay
  ;[1 1 1] Set the default values
  (Variables|Default|SetWanderDestination (Transformation|GetActorLocation self))
  (bind _returnvalue (AddComponent|AddAudioComponent false))
  (bind _output_get (Variables|Default|SetOstricheNoise _returnvalue))
  (Audio|Components|Audio|SetSound _output_get "/Game/Audio/OstrichRoar.OstrichRoar"))

(fn ConstructionScript)

(fn RaycastforPlayer
  (params (Start :type Vector) (End :type Vector) (OtherActor :type Actor%20Object%20Reference))
  (bind _outactors (Actor|GetAllActorsOfClass "EnemyOstrich_C"))
  (bind _returnvalue (Collision|LineTraceByChannel Start End "TraceTypeQuery1" false _outactors "ForOneFrame"))
  (return (or (>= (Transformation|GetDistanceTo OtherActor) 1.5e+03) _returnvalue)))

(fn Wander
  (params (B :type Float%20%28single-precision%29))
  (bind _self self)
  (bind _playerdetected (Variables|Default|GetPlayerDetected))
  (bind _playerpursuit (Variables|Default|GetPlayerPursuit))
  (bind _returnvalue (Math|Boolean|NORBoolean _playerdetected _playerpursuit))
  (bind _returnvalue_2 (Transformation|GetActorLocation _self))
  ;[1 1 1] Cause the enemy to wander around the navmesh, decrease the walk speed to
  (if (Math|Boolean|ANDBoolean (<= (Math|Vector|VectorLength (- (Variables|Default|GetWanderDestination) _returnvalue_2)) 1e+02) _returnvalue (>= (Variables|Default|GetRestTimer) 5.0))
    (if (and (>= (Math|Random|RandomInteger 100) 50) (>= (Variables|Default|GetRestTimer) 5.0))
      (bind _output_get (Variables|Default|SetWanderDestination (AI|Navigation|GetRandomReachablePointinRadius _returnvalue_2 1e+03)))
      (Variables|Default|SetRestTimer 5.0)
      (AI|Navigation|SimpleMovetoLocation (Pawn|GetController) _output_get :!label _label)
      (Variables|/Script/Engine.CharacterMovementComponent|SetMaxWalkSpeed (Variables|Character|GetCharacterMovement) (Variables|Default|GetCalmMovementSpeed))
      (bind _output_get_2 (Variables|Default|SetRestTimer (+ (stale _output_get_2) B)))
      (else
        (Variables|Default|SetRestTimer (Math|Random|RandomFloatinRange 0.0 3.0))))
    (elif _returnvalue
      (goto _label))))

(fn EnemyDetection
  (bind _self self)
  (bind _returnvalue (Transformation|GetActorLocation _self))
  ;[1 1 1] Get the angle between the facing of the enemy and the player. If the angle is small enough begin to pursue the player
  (if (Math|Boolean|NORBoolean (Variables|Default|GetPlayerDetected) (Variables|Default|GetPlayerPursuit))
    (bind _ascharacter (Utilities|Casting|CastToCharacter (Game|Player|GetPlayerPawn 0)))
    (bind _returnvalue_2 (CallFunction|RaycastforPlayer _returnvalue (Transformation|GetActorLocation _ascharacter) _ascharacter))
    (if (Math|Boolean|ANDBoolean (>= (Math|Vector|DotProduct (Math|Vector|Normalize (- (Transformation|GetActorLocation _ascharacter) _returnvalue)) (Math|Vector|GetForwardVector (Transformation|GetActorRotation _self))) (Math|Trig|Cos(Degrees) 45.0)) (>= 9e+02 (Transformation|GetDistanceTo _ascharacter)) true)
      (Variables|Default|SetPlayerDetected true)
      (Variables|Default|SetPlayerPursuit true)
      (Variables|Default|SetDisinterestTime 0.0)
      (Variables|/Script/Engine.CharacterMovementComponent|SetMaxWalkSpeed (Variables|Character|GetCharacterMovement) (Variables|Default|GetPursuitMovementSpeed))
      (Audio|Components|Audio|Play (Variables|Default|GetOstricheNoise) 0.0))))

(fn PursueVisibleEnemy
  (params (B :type Float%20%28single-precision%29))
  ;[1 1 1] While a raycast can reach the player, pursue the position of the player. When the Player breaks LOS, the enemy will pursue the last known location
  (if (and (Variables|Default|GetPlayerPursuit) (Variables|Default|GetPlayerDetected))
    (Variables|/Script/Engine.CharacterMovementComponent|SetMaxWalkSpeed (Variables|Character|GetCharacterMovement) (Variables|Default|GetPursuitMovementSpeed))
    (bind _ascharacter (Utilities|Casting|CastToCharacter (Game|Player|GetPlayerPawn 0)))
    (bind _returnvalue (CallFunction|RaycastforPlayer (Transformation|GetActorLocation self) (Transformation|GetActorLocation _ascharacter) _ascharacter))
    (if _returnvalue
      (Variables|Default|SetPlayerDetected false)
      (else
        (bind _output_get (Variables|Default|SetPlayerPosition (Transformation|GetActorLocation _ascharacter)))
        (Variables|Default|SetDisinterestTime 0.0)
        (AI|Navigation|SimpleMovetoLocation (Pawn|GetController) _output_get)
        (if (<= (Math|Vector|VectorLength (- (Transformation|GetActorLocation _ascharacter) (Transformation|GetActorLocation self))) 3e+02)
          (bind _output_get_2 (Variables|Default|SetAttackTimer (+ (stale _output_get_2) B)))
          (if (>= _output_get_2 2.0)
            (Variables|Default|SetAttackTimer 0.0)
            (if (Collision|IsOverlappingActor (Variables|Default|GetAttackTrigger) _ascharacter :!class /Script/Engine.PrimitiveComponent)
              (Character|LaunchCharacter _ascharacter (* (Math|Vector|Normalize (+ (Math|Vector|GetForwardVector (Transformation|GetActorRotation self)) "0, 0,1.000000")) 5e+02) true true)
              (Development|PrintString "Attack Damage Here"))))))))

(fn PursueLastKnownLocation
  (params (B :type Float%20%28single-precision%29))
  (bind _self self)
  (bind _returnvalue (Transformation|GetActorLocation _self))
  ;[1 1 1] Handles movement  and player detection, when the user is in sight continue the chase, if the user is hidden for 3 seconds
  (if (and (Variables|Default|GetPlayerPursuit) (not (Variables|Default|GetPlayerDetected)))
    (bind _ascharacter (Utilities|Casting|CastToCharacter (Game|Player|GetPlayerPawn 0)))
    (bind _returnvalue_2 (CallFunction|RaycastforPlayer (Transformation|GetActorLocation self) (Transformation|GetActorLocation _ascharacter) _ascharacter))
    (AI|Navigation|SimpleMovetoLocation (Pawn|GetController) (Variables|Default|GetPlayerPosition))
    (if _returnvalue_2
      (if (and (not (Variables|Default|GetPlayerDetected)) (<= (Math|Vector|VectorLength (- (Variables|Default|GetPlayerPosition) _returnvalue)) 5e+01))
        (Variables|Default|SetPlayerPursuit false :!label _label)
        (Variables|Default|SetWanderDestination (AI|Navigation|GetRandomReachablePointinRadius (Transformation|GetActorLocation self) 1e+03))
        (else
          (bind _output_get (Variables|Default|SetDisinterestTime (+ (Variables|Default|GetDisinterestTime) B)))
          (Transformation|SetActorRotation (Math|Rotator|MakeRotator 0.0 0.0 (.Yaw (Math|Rotator|BreakRotator (Math|Rotator|FindLookatRotation _returnvalue (Variables|Default|GetPlayerPosition))))))
          (if (> _output_get 8.0)
            (goto _label))))
      (else
        (Variables|Default|SetPlayerDetected true)
        (Variables|Default|SetPlayerPosition (Variables|Default|GetPlayerPosition))
        (Variables|Default|SetDisinterestTime 0.0)))))

(fn CalculateMorale
  (bind _self self)
  (Variables|Default|SetMorale 0)
  (Variables|Default|SetAlliesInRange 0)
  (bind _outactors (Actor|GetAllActorsOfClass "EnemyOstrich_C"))
  (for _array_element _outactors
    (if (<= (Transformation|GetDistanceTo _array_element self) 1e+03)
      (bind _output_get (Variables|EnemyOstrich_C|SetPlayerDetected _array_element (or (stale _output_get) (Variables|Default|GetPlayerDetected _self))))
      (bind _output_get_2 (Variables|EnemyOstrich_C|SetPlayerPursuit _array_element (or (Variables|Default|GetPlayerPursuit _self) (stale _output_get_2))))
      (bind _output_get_3 (Variables|Default|SetMorale (+ (Variables|EnemyOstrich_C|GetHealth _array_element) (stale _output_get_3))))
      (Math|Integer|IncrementInt (Variables|Default|GetAlliesInRange))))
  (if (not (> _output_get_3 (* (Variables|Default|GetAlliesInRange) 5)))
    (Variables|Default|SetFleeing true)))

(fn CalculateFleeTime
  (params (A :type Float%20%28single-precision%29))
  (bind _output_get (Variables|Default|SetFleeTimer (+ A (stale _output_get))))
  (if (>= _output_get 3e+01)
    (Variables|Default|SetFleeTimer 0.0)
    (Variables|Default|SetHealth (Variables|Default|GetMaxHealth))
    (Variables|Default|SetFleeing false)))

(fn Flee
  (bind _self self)
  (bind _returnvalue (Transformation|GetActorLocation _self))
  ;[1 1 1] Check if the player is in sight if so runaway
  (if (Variables|Default|GetPlayerPursuit)
    (Variables|/Script/Engine.CharacterMovementComponent|SetMaxWalkSpeed (Variables|Character|GetCharacterMovement) (Variables|Default|GetPursuitMovementSpeed))
    (bind _ascharacter (Utilities|Casting|CastToCharacter (Game|Player|GetPlayerPawn 0)))
    (bind _returnvalue_2 (CallFunction|RaycastforPlayer _returnvalue (Transformation|GetActorLocation _ascharacter) _ascharacter))
    (if _returnvalue_2
      (Variables|Default|SetWanderDestination (AI|Navigation|GetRandomReachablePointinRadius (Transformation|GetActorLocation self) 1e+03))
      (Variables|Default|SetPlayerDetected false)
      (Variables|Default|SetPlayerPursuit false)
      (else
        (bind _output_get (Variables|Default|SetPlayerPosition (Transformation|GetActorLocation _ascharacter)))
        (AI|Navigation|SimpleMovetoLocation (Pawn|GetController) (+ (* (Math|Vector|Normalize (- _returnvalue _output_get)) 250) _returnvalue))))))

(fn Damage
  (params (Damage :type Integer))
  (Variables|Default|SetPlayerPursuit true)
  (Character|LaunchCharacter (* (Math|Vector|Normalize (+ (Math|Vector|GetForwardVector (Transformation|GetActorRotation (Game|GetPlayerCharacter 0))) "0, 0,1.000000")) 5e+02) true true)
  (bind _output_get (Variables|Default|SetHealth (- (stale _output_get) Damage))))