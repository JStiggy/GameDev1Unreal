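; LadderVolume is a trigger volume that lets the player climb while inside its overlap area.
; On overlap it enables its own input and zeroes the player's gravity scale, then reverses both on exit.
; Pressing Space inside starts a Delay-based loop that sets Flying mode and adds upward movement input while the key is held.
; The loop restores Walking mode once Space is released or the player leaves.
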(event OnComponentBeginOverlap(LadderOverlapArea)
  (params (OverlappedComponent :type Primitive%20Component%20Object%20Reference) (OtherActor :type Actor%20Object%20Reference) (OtherComp :type Primitive%20Component%20Object%20Reference) (OtherBodyIndex :type Integer) (bFromSweep :type Boolean) (SweepResult :type Hit%20Result%20Structure%20%28by%20ref%29))
  (bind _returnvalue (Game|Player|GetPlayerPawn 0))
  (if (== OtherActor _returnvalue)
    (bind _asplayer_controller (Utilities|Casting|CastToPlayerController (Pawn|GetController _returnvalue)))
    (Input|EnableInput _asplayer_controller)
    (Variables|Default|SetUsing true)
    (Variables|/Script/Engine.CharacterMovementComponent|SetGravityScale (Variables|/Script/Engine.Character|GetCharacterMovement (Game|GetPlayerCharacter 0)) 0.0)))

(event OnComponentEndOverlap(LadderOverlapArea)
  (params (OverlappedComponent :type Primitive%20Component%20Object%20Reference) (OtherActor :type Actor%20Object%20Reference) (OtherComp :type Primitive%20Component%20Object%20Reference) (OtherBodyIndex :type Integer))
  (bind _returnvalue (Game|Player|GetPlayerPawn 0))
  (if (== OtherActor _returnvalue)
    (bind _asplayer_controller (Utilities|Casting|CastToPlayerController (Pawn|GetController _returnvalue)))
    (Input|DisableInput _asplayer_controller)
    (Variables|Default|SetUsing false)
    (Variables|/Script/Engine.CharacterMovementComponent|SetGravityScale (Variables|/Script/Engine.Character|GetCharacterMovement (Game|GetPlayerCharacter 0)) 1.0)))

(event Input|AxisEvents|InputAxisMoveRight
  (params (AxisValue :type Float%20%28single-precision%29)))

(event Input|KeyboardEvents|SpaceBar
  (params (Key :type Key%20Structure :default "AnyKey"))
  (bind _returnvalue (Game|Player|GetPlayerPawn 0))
  (bind _returnvalue_2 (Game|GetPlayerCharacter 0))
  (bind _charactermovement (Variables|/Script/Engine.Character|GetCharacterMovement _returnvalue_2))
  (:Pressed
    (if (Variables|Default|GetUsing) :!label _label
      (if (Game|Player|IsInputKeyDown (Game|GetPlayerController 0) "SpaceBar")
        (Pawn|Components|CharacterMovement|SetMovementMode _charactermovement "MOVE_Flying" 0)
        (Pawn|Input|AddMovementInput _returnvalue (Transformation|GetActorUpVector _returnvalue) 1e+02 false)
        (Utilities|FlowControl|Delay 0.2)
        (goto _label)
        (else
          _)))
    (Pawn|Components|CharacterMovement|SetMovementMode _charactermovement "MOVE_Walking" 0)))

(fn ConstructionScript)