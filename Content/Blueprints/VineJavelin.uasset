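; Vine Javelin is a short-lived attack actor that tethers to the first-person player with a cable and damages Enemy Ostriches it touches.
; It zeroes the player's walk speed on BeginPlay, then restores a hardcoded speed and prints a placeholder spawn message when destroyed.
; A box overlap knocks the ostrich forward and up, decrements its health, triggers pursuit with a target position depending on fleeing state, then destroys the javelin.
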(event OnComponentBeginOverlap(Box)
  (params (OverlappedComponent :type Primitive%20Component%20Object%20Reference) (OtherActor :type Actor%20Object%20Reference) (OtherComp :type Primitive%20Component%20Object%20Reference) (OtherBodyIndex :type Integer) (bFromSweep :type Boolean) (SweepResult :type Hit%20Result%20Structure%20%28by%20ref%29))
  (bind _asenemy_ostrich (Utilities|Casting|CastToEnemyOstrich OtherActor))
  (CallFunction|OstrichHit _asenemy_ostrich))

(event EventBeginPlay
  ;[1 1 1] Set information for the Vine Javelin
  (Actor|SetLifeSpan 2.0)
  (bind _asfirst_person_character (Utilities|Casting|CastToFirstPersonCharacter (Game|Player|GetPlayerPawn 0)))
  (Class|CableComponent|SetAttachEndto (Variables|Default|GetCable) _asfirst_person_character "None")
  (Variables|/Script/Engine.CharacterMovementComponent|SetMaxWalkSpeed (Variables|/Script/Engine.Character|GetCharacterMovement _asfirst_person_character) 0.0))

(event EventDestroyed
  ;[1 1 1] Set information for the Vine Javelin
  (Variables|/Script/Engine.CharacterMovementComponent|SetMaxWalkSpeed (Variables|/Script/Engine.Character|GetCharacterMovement (stale EventBeginPlay _asfirst_person_character)) 6e+02)
  (Development|PrintString "Spawn a Vine Javelin here"))

(fn ConstructionScript)

(fn OstrichHit
  (params (NewParam :type Enemy%20Ostrich%20Object%20Reference))
  (Variables|/Game/Blueprints/EnemyOstrich.EnemyOstrich_C|SetPlayerPursuit NewParam true)
  (Character|LaunchCharacter NewParam (* (Math|Vector|Normalize (+ (Math|Vector|GetForwardVector (Transformation|GetActorRotation self)) "0, 0,1.000000")) 5e+02) true true)
  (bind _output_get (Variables|/Game/Blueprints/EnemyOstrich.EnemyOstrich_C|SetHealth NewParam (- (stale _output_get) 1)))
  (if (Variables|/Game/Blueprints/EnemyOstrich.EnemyOstrich_C|GetFleeing NewParam)
    (Variables|/Game/Blueprints/EnemyOstrich.EnemyOstrich_C|SetPlayerPosition NewParam (Transformation|GetActorLocation))
    (else
      (Variables|/Game/Blueprints/EnemyOstrich.EnemyOstrich_C|SetPlayerPosition NewParam (Transformation|GetActorLocation (Game|GetPlayerCharacter 0)))))
  (Actor|DestroyActor))