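; Fire javelin projectile that damages EnemyOstrich characters and scares them into fleeing.
; Every Tick it scans all ostriches and sets any within a short radius to flee on a timer.
; On box overlap, OstrichHit deals damage, launches the ostrich forward and up, updates its pursuit target and destroys the javelin, then the ostrich is set fleeing.
; A blocking hit on the box instead starts a short lifespan countdown.
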(event OnComponentBeginOverlap(Box)
  (params (OverlappedComponent :type Primitive%20Component%20Object%20Reference) (OtherActor :type Actor%20Object%20Reference) (OtherComp :type Primitive%20Component%20Object%20Reference) (OtherBodyIndex :type Integer) (bFromSweep :type Boolean) (SweepResult :type Hit%20Result%20Structure%20%28by%20ref%29))
  (bind _asenemy_ostrich (Utilities|Casting|CastToEnemyOstrich OtherActor))
  (CallFunction|OstrichHit _asenemy_ostrich)
  (Variables|/Game/Blueprints/EnemyOstrich.EnemyOstrich_C|SetFleeing _asenemy_ostrich true)
  (Variables|/Game/Blueprints/EnemyOstrich.EnemyOstrich_C|SetFleeTimer _asenemy_ostrich 2e+01))

(event OnComponentHit(Box)
  (params (HitComponent :type Primitive%20Component%20Object%20Reference) (OtherActor :type Actor%20Object%20Reference) (OtherComp :type Primitive%20Component%20Object%20Reference) (NormalImpulse :type Vector :default "0, 0, 0") (Hit :type Hit%20Result%20Structure%20%28by%20ref%29))
  (Actor|SetLifeSpan 6.0))

(event EventTick
  (params (DeltaSeconds :type Float%20%28single-precision%29))
  (bind _outactors (Actor|GetAllActorsOfClass "/Game/Blueprints/EnemyOstrich.EnemyOstrich_C"))
  (for _array_element _outactors
    (if (< (Transformation|GetDistanceTo _array_element self) 3e+02)
      (Variables|/Game/Blueprints/EnemyOstrich.EnemyOstrich_C|SetFleeing _array_element true)
      (Variables|/Game/Blueprints/EnemyOstrich.EnemyOstrich_C|SetFleeTimer _array_element 25.0))))

(fn ConstructionScript)

(fn OstrichHit
  (params (NewParam :type Enemy%20Ostrich%20Object%20Reference))
  (Variables|/Game/Blueprints/EnemyOstrich.EnemyOstrich_C|SetPlayerPursuit NewParam true)
  (Character|LaunchCharacter NewParam (* (Math|Vector|Normalize (+ (Math|Vector|GetForwardVector (Transformation|GetActorRotation self)) "0, 0,1.000000")) 5e+02) true true)
  (bind _output_get (Variables|/Game/Blueprints/EnemyOstrich.EnemyOstrich_C|SetHealth NewParam (- (stale _output_get) 3)))
  (if (Variables|/Game/Blueprints/EnemyOstrich.EnemyOstrich_C|GetFleeing NewParam)
    (Variables|/Game/Blueprints/EnemyOstrich.EnemyOstrich_C|SetPlayerPosition NewParam (Transformation|GetActorLocation))
    (else
      (Variables|/Game/Blueprints/EnemyOstrich.EnemyOstrich_C|SetPlayerPosition NewParam (Transformation|GetActorLocation (Game|GetPlayerCharacter 0)))))
  (Actor|DestroyActor))